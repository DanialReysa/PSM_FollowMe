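; PuzzleItem_BP is a collectible puzzle item that reports its pickup to PuzzleGate_BP.
; When ThirdPersonCharacter overlaps its Trigger, it enables input for player controller 0 and prints a "Collect" prompt.
; Pressing F looks up the gate with GetActorOfClass, calls CollectItem on it and destroys the item.
; DisableInput is unwired from the end-overlap event, so F stays active after the player leaves.
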(event `Key|F`
  (params (Key :type "Key Structure"))
  (:`Pressed`
    (bind _returnvalue (`GameplayStatics.GetActorOfClass` "/Game/FollowMeLibrary/Mechanic/MainDoor/PuzzleGate_BP.PuzzleGate_BP_C"))
    (`/Game/FollowMeLibrary/Mechanic/MainDoor/PuzzleGate_BP.Collect Item` _returnvalue)
    (`self.K2_DestroyActor`)))

(event `self.Trigger.OnComponentBeginOverlap`
  (params (OverlappedComponent :type "PrimitiveComponent Object Reference") (OtherActor :type "Actor Object Reference") (OtherComp :type "PrimitiveComponent Object Reference") (OtherBodyIndex :type Integer) (bFromSweep :type Boolean) (SweepResult :type "HitResult Structure (by ref)"))
  (cast `/Game/FollowMeLibrary/Player/ThirdPersonCharacter` OtherActor)
  (`self.EnableInput` (`GameplayStatics.GetPlayerController` 0))
  (`KismetSystemLibrary.PrintString` "Collect"))

(event `self.Trigger.OnComponentEndOverlap`
  (params (OverlappedComponent :type "PrimitiveComponent Object Reference") (OtherActor :type "Actor Object Reference") (OtherComp :type "PrimitiveComponent Object Reference") (OtherBodyIndex :type Integer))
  (cast `/Game/FollowMeLibrary/Player/ThirdPersonCharacter` OtherActor))

(fn `UserConstructionScript`)