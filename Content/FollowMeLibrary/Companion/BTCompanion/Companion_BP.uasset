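; Companion character that follows, waits, moves to targets, assists the player, leads to a checkpoint or wanders searching.
; Wait, Follow and MoveToTarget set state on Companion_AI, while Assisting, LeadTheWay and looping Searching call AIMoveTo directly, most with their own walk speed.
; Seeing a StaticEnemyAI freezes movement until a retriggerable three-second delay ends.
; A hard landing ragdolls it, fades the screen and reloads the level.
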(event `self.ReceiveBeginPlay`
  ;[1 1 1] Comment
  (`|ExecutionSequence`
    (:`then_0`
      (bind _ascompanion_ai (cast `/Game/FollowMeLibrary/Companion/BTCompanion/Companion_AI` (`AIBlueprintHelperLibrary.GetAIController` self)))
      (set `self.CompanionController` _ascompanion_ai))
    (:`then_1`
      (bind _asthird_person_character (cast `/Game/FollowMeLibrary/Player/ThirdPersonCharacter` (`GameplayStatics.GetPlayerCharacter` 0)))
      (set `self.Player REF` _asthird_person_character))
    (:`then_2`
      (bind _outactors (`GameplayStatics.GetAllActorsOfClass` "/Game/FollowMeLibrary/Enemy/StaticEnemyAI.StaticEnemyAI_C"))
      (set `self.SeeEnemy` (`|GetArrayItem` _outactors)))))

(event `Wait`
  ;[1 1 1] Comment
  (`/Game/FollowMeLibrary/Companion/BTCompanion/Companion_AI.SetCompanionState` (`self.CompanionController`) "NewEnumerator0"))

(event `Follow`
  (params (FollowTarget :type "Actor Object Reference"))
  ;[1 1 1] Comment
  (set `CharacterMovementComponent.MaxWalkSpeed` 250.0 (`self.CharacterMovement`))
  (`self.UnCrouch`)
  (`/Game/FollowMeLibrary/Companion/BTCompanion/Companion_AI.SetFollowActor` (`self.CompanionController`) FollowTarget)
  (`/Game/FollowMeLibrary/Companion/BTCompanion/Companion_AI.SetCompanionState` (`self.CompanionController`) "NewEnumerator1"))

(event `MoveToTarget`
  (params (Location :type "Vector Structure"))
  ;[1 1 1] Comment
  (set `CharacterMovementComponent.MaxWalkSpeed` 500.0 (`self.CharacterMovement`))
  (`/Game/FollowMeLibrary/Companion/BTCompanion/Companion_AI.SetTargetLocation` (`self.CompanionController`) Location)
  (`/Game/FollowMeLibrary/Companion/BTCompanion/Companion_AI.SetCompanionState` (`self.CompanionController`) "NewEnumerator0")
  (`/Game/FollowMeLibrary/Companion/BTCompanion/Companion_AI.SetCompanionState` (`self.CompanionController`) "NewEnumerator2"))

(event `self.OnLanded`
  (params (Hit :type "HitResult Structure (by ref)"))
  (bind (_returnvalue_x _returnvalue_y _returnvalue_z) (`KismetMathLibrary.BreakVector` (`self.GetVelocity`)))
  ;[1 1 1] Fall on Impact https://youtu.be/C_EaLJVY1XQ?si=ksi6aNzmbEfl9zkI
  (if (> (`KismetMathLibrary.Abs` _returnvalue_z) 800.0)
    (`KismetSystemLibrary.PrintString` "Dead")
    (`PrimitiveComponent.SetSimulatePhysics` (`self.Mesh`) true)
    (`PrimitiveComponent.AddImpulse` (`self.Mesh`) (0.0 0.0 5000.0) "None" false)
    (`CharacterMovementComponent.DisableMovement` (`self.CharacterMovement`))
    (`GameplayStatics.PlaySound2D` "/Engine/VREditor/Sounds/UI/Click_on_Button.Click_on_Button" 1.0 1.0 0.0 null null)
    (bind _returnvalue (`|CreateWidget` "/Game/FollowMeLibrary/Widget/LevelTransfer/Fade.Fade_C"))
    (`UserWidget.AddToViewport` _returnvalue 0)
    (`/Game/FollowMeLibrary/Widget/LevelTransfer/Fade.Fade Anim` _returnvalue)
    (`KismetSystemLibrary.Delay` 2.0)
    (bind _returnvalue_2 (`GameplayStatics.GetCurrentLevelName` true))
    (`GameplayStatics.OpenLevel` (`KismetStringLibrary.Conv_StringToName` _returnvalue_2))))

(event `Assisting`
  (set `CharacterMovementComponent.MaxWalkSpeed` 500.0 (`self.CharacterMovement`))
  (`|AIMoveTo` self (0.0 0.0 0.0) (`self.Player REF`)
    (:`OnSuccess`
      (`self.PlayAnimMontage` "/Game/FollowMeLibrary/SpecialAnimation/Assisting/Assisting_UE_Montage.Assisting_UE_Montage"))))

(event `LeadTheWay`
  (set `CharacterMovementComponent.MaxWalkSpeed` 240.0 (`self.CharacterMovement`))
  (`|AIMoveTo` self (0.0 0.0 0.0) (`self.Checkpoint`)))

(event `Searching`
  (set `CharacterMovementComponent.MaxWalkSpeed` 300.0 (`self.CharacterMovement`))
  (`|AIMoveTo` self (`NavigationSystemV1.K2_GetRandomReachablePointInRadius` (`self.K2_GetActorLocation`) 1200.0 null null) null
    (:`OnSuccess`
      (`KismetSystemLibrary.Delay` 2.0)
      (`self.Searching`))))

(event `self.PawnSensing.OnSeePawn`
  (params (Pawn :type "Pawn Object Reference"))
  (bind _charactermovement (`self.CharacterMovement`))
  (cast `/Game/FollowMeLibrary/Enemy/StaticEnemyAI` Pawn)
  (`|ExecutionSequence`
    (:`then_0`
      (`CharacterMovementComponent.DisableMovement` _charactermovement))
    (:`then_1`
      (`KismetSystemLibrary.RetriggerableDelay` 3.0)
      (`CharacterMovementComponent.SetMovementMode` _charactermovement "MOVE_Walking" 0))))

(fn `UserConstructionScript`)