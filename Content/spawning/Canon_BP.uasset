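; Canon_BP is a hazard actor that damages the player's ThirdPersonCharacter when it overlaps the collision sphere.
; It caches the player character at BeginPlay, then subtracts a fixed amount from its HealthValue on overlap, with a DoOnce and Delay acting as a damage cooldown.
; Each valid overlap also plays a backwards hit-reaction montage if health equals exactly zero.
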(event `self.ReceiveBeginPlay`
  ;[1 1 1] Comment
  (bind _asthird_person_character (cast `/Game/FollowMeLibrary/Player/ThirdPersonCharacter` (`GameplayStatics.GetPlayerCharacter` 0)))
  (set `self.Camilla REF` _asthird_person_character))

(event `self.CollisionSphere.OnComponentBeginOverlap`
  (params (OverlappedComponent :type "PrimitiveComponent Object Reference") (OtherActor :type "Actor Object Reference") (OtherComp :type "PrimitiveComponent Object Reference") (OtherBodyIndex :type Integer) (bFromSweep :type Boolean) (SweepResult :type "HitResult Structure (by ref)"))
  (bind _camilla_ref (`self.Camilla REF`))
  ;[1 1 1] Comment
  (cast `/Game/FollowMeLibrary/Player/ThirdPersonCharacter` OtherActor)
  (`|ExecutionSequence`
    (:`then_0`
      (`/Engine/EditorBlueprintResources/StandardMacros.DoOnce` false :!label _label
        (:`Completed`
          (set `/Game/FollowMeLibrary/Player/ThirdPersonCharacter.Health Value` (- (`/Game/FollowMeLibrary/Player/ThirdPersonCharacter.Health Value` _camilla_ref) 10.0) _camilla_ref)
          (`KismetSystemLibrary.Delay` 2.0)
          (goto _label :!via `Reset`))))
    (:`then_1`
      (if (== (`/Game/FollowMeLibrary/Player/ThirdPersonCharacter.Health Value` (`self.Camilla REF`)) 0.0)
        (`Character.PlayAnimMontage` (`self.Camilla REF`) "/Game/FollowMeLibrary/PlatformerBoy/EnemyChaser/Finisher/GettingHitBackwards_UE_Montage.GettingHitBackwards_UE_Montage" 1.0 "None")))))

(fn `UserConstructionScript`)